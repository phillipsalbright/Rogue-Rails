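; Equippable held-body item that lets the player carry an enemy guard's body and throw it.
; Action plays a first-person throw montage.
; ExecuteThrow spawns a body pickup with new item data, unequips, and spawns a fresh guard, killing it immediately and attaching the pickup to it.
; It then removes the body from inventory, destroys itself and launches the ragdoll along the camera's forward vector.
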(fn `Action`
  (`parent.Action`)
  (`AnimInstance.Montage_Play` (`SkeletalMeshComponent.GetAnimInstance` (`/Game/Blueprints/Characters/BP_RRCharacter.FirstPersonMesh` (`self.Player Char`))) "/Game/Models/Arms/AM_Throw.AM_Throw" 1.2 "MontageLength" 0.0 true))

(fn `ExecuteThrow`
  (bind _bp_inventorycomponent (`/Game/Blueprints/Characters/BP_RRCharacter.BP_InventoryComponent` (`self.Player Char`)))
  (bind _firstpersoncamera (`/Game/Blueprints/Characters/BP_RRCharacter.FirstPersonCamera` (`self.Player Char`)))
  (bind _returnvalue (`SceneComponent.GetForwardVector` _firstpersoncamera))
  (bind _returnvalue_2 (`|GenericCreateObject` "/Game/Blueprints/Items/BP_ItemObject.BP_ItemObject_C" (make `IntPoint` 4 2) "/Game/Materials/M_IconBody.M_IconBody" "/Game/Materials/M_IconBody_Rotated.M_IconBody_Rotated" "/Game/Blueprints/Items/BP_Body.BP_Body_C" true "BP_BodyHeld_C" "Body"))
  (bind _returnvalue_3 (`|SpawnActorFromClass` "/Game/Blueprints/Items/BP_Body.BP_Body_C" (`KismetMathLibrary.MakeTransform` (+ (`SceneComponent.K2_GetComponentLocation` _firstpersoncamera) (* _returnvalue 100.0))) "Undefined" "MultiplyWithRoot" null _returnvalue_2 null))
  (`/Game/Blueprints/Characters/BP_RRCharacter.Unequip` (`self.Player Char`))
  (bind _returnvalue_4 (`|SpawnActorFromClass` "/Game/Blueprints/Characters/BP_EnemyGuard.BP_EnemyGuard_C" (`self.GetTransform` _returnvalue_3) "Undefined" "MultiplyWithRoot" _returnvalue_3 null))
  (`/Engine/EditorBlueprintResources/StandardMacros.IsValid` _returnvalue_4
    (:`Is Valid`
      (`self.K2_AttachToComponent` _returnvalue_3 (`/Game/Blueprints/Characters/BP_EnemyGuard.PickupAnchor` _returnvalue_4) "None" "SnapToTarget" "SnapToTarget" "KeepRelative" true)
      (bind _output_get (set `/Game/Blueprints/Items/BP_Body.AttachedEnemy` _returnvalue_4 _returnvalue_3))
      (`/Game/Blueprints/Characters/BP_EnemyGuard.Death` _output_get)
      (bind _itemobject (`/Game/Blueprints/Inventory/BP_InventoryComponent.GetItemOfType` _bp_inventorycomponent "/Game/Blueprints/Items/BP_Body.BP_Body_C"))
      (`/Game/Blueprints/Inventory/BP_InventoryComponent.RemoveItem` _bp_inventorycomponent _itemobject)
      (`self.K2_DestroyActor`)
      (bind _mesh (`Character.Mesh` _output_get))
      (`PrimitiveComponent.SetSimulatePhysics` _mesh true)
      (`PrimitiveComponent.AddImpulse` _mesh (* _returnvalue 8000.0) "None" true))))

(fn `UserConstructionScript`
  (`parent.UserConstructionScript`))