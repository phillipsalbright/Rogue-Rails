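; BP_Lockpick is an equippable lockpick that unlocks BP_UnlockableObject actors in front of the player.
; Action plays a use montage on the first-person mesh and line-traces a short distance from the camera, leaving persistent debug lines.
; A hit on an unlockable calls Unlock, unequips the player and removes a lockpick pickup from the inventory.
; A Tick-driven cooldown, named KnifeCooldown, limits reuse.
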(event `self.ReceiveTick`
  (params (DeltaSeconds :type "Float (single-precision)"))
  (`parent.ReceiveTick` DeltaSeconds)
  (if (> (`self.KnifeCooldown`) 0.0)
    (set `self.KnifeCooldown` (- (`self.KnifeCooldown`) DeltaSeconds))))

(fn `Action`
  (bind _player_char (`self.Player Char`))
  (bind _firstpersoncamera (`/Game/Blueprints/Characters/BP_RRCharacter.FirstPersonCamera` (`self.Player Char`)))
  (bind _bp_inventorycomponent (`/Game/Blueprints/Characters/BP_RRCharacter.BP_InventoryComponent` _player_char))
  (bind _returnvalue (`SceneComponent.K2_GetComponentLocation` _firstpersoncamera))
  (`parent.Action`)
  (if (<= (`self.KnifeCooldown`) 0.0)
    (`AnimInstance.Montage_Play` (`SkeletalMeshComponent.GetAnimInstance` (`/Game/Blueprints/Characters/BP_RRCharacter.FirstPersonMesh` (`self.Player Char`))) "/Game/Models/Arms/AM_UseObject.AM_UseObject" 1.5 "MontageLength" 0.0 true)
    (set `self.KnifeCooldown` 1.0)
    (bind _outhit (`KismetSystemLibrary.LineTraceSingle` :`Start` _returnvalue :`End` (+ _returnvalue (* (`SceneComponent.GetForwardVector` _firstpersoncamera) 210.0)) :`TraceChannel` "TraceTypeQuery1" :`DrawDebugType` "Persistent"))
    (bind _asbp_unlockable_object (cast `/Game/Blueprints/Lockpick/BP_UnlockableObject` (`.HitActor` (`GameplayStatics.BreakHitResult` _outhit))))
    (`/Game/Blueprints/Lockpick/BP_UnlockableObject.Unlock` _asbp_unlockable_object)
    (`/Game/Blueprints/Characters/BP_RRCharacter.Unequip` _player_char)
    (bind _itemobject (`/Game/Blueprints/Inventory/BP_InventoryComponent.GetItemOfType` _bp_inventorycomponent "/Game/Blueprints/Items/BP_LockpickPickup.BP_LockpickPickup_C"))
    (if (`KismetSystemLibrary.IsValid` _itemobject)
      (`/Game/Blueprints/Inventory/BP_InventoryComponent.RemoveItem` _bp_inventorycomponent _itemobject))))

(fn `UserConstructionScript`
  (`parent.UserConstructionScript`))