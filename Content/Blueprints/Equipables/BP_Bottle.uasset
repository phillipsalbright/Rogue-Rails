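; Equippable bottle that the player throws from first person, with its Action playing a throw montage on the first-person mesh.
; ExecuteThrow, triggered from outside this file, spawns a breakable bottle ahead of the camera and launches it with a velocity-change impulse on its Geometry Collection.
; It then unequips the bottle and removes a matching pickup from the inventory.
; An older static-mesh throw remains disconnected in Action.
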(fn `Action`
  (`parent.Action`)
  (`AnimInstance.Montage_Play` (`SkeletalMeshComponent.GetAnimInstance` (`/Game/Blueprints/Characters/BP_RRCharacter.FirstPersonMesh` (`self.Player Char`))) "/Game/Models/Arms/AM_Throw.AM_Throw" 1.2 "MontageLength" 0.0 true))

(fn `ExecuteThrow`
  (bind _player_char (`self.Player Char`))
  (bind _firstpersoncamera (`/Game/Blueprints/Characters/BP_RRCharacter.FirstPersonCamera` (`self.Player Char`)))
  (bind _bp_inventorycomponent (`/Game/Blueprints/Characters/BP_RRCharacter.BP_InventoryComponent` _player_char))
  (bind _returnvalue (`SceneComponent.GetForwardVector` _firstpersoncamera))
  (bind _returnvalue_2 (`|SpawnActorFromClass` "/Game/Blueprints/LevelObjects/BP_BottleThrownBreaks.BP_BottleThrownBreaks_C" (`KismetMathLibrary.MakeTransform` (+ (`SceneComponent.K2_GetComponentLocation` _firstpersoncamera) (* _returnvalue 100.0))) "Undefined" "MultiplyWithRoot" null null))
  (`PrimitiveComponent.AddImpulse` (`self.GetComponentByClass` _returnvalue_2 "/Script/GeometryCollectionEngine.GeometryCollectionComponent") (* _returnvalue 1500.0) "None" true)
  (`/Game/Blueprints/Characters/BP_RRCharacter.Unequip` _player_char)
  (bind _itemobject (`/Game/Blueprints/Inventory/BP_InventoryComponent.GetItemOfType` _bp_inventorycomponent "/Game/Blueprints/Items/BP_BottlePickup.BP_BottlePickup_C"))
  (if (`KismetSystemLibrary.IsValid` _itemobject)
    (`/Game/Blueprints/Inventory/BP_InventoryComponent.RemoveItem` _bp_inventorycomponent _itemobject)))

(fn `UserConstructionScript`
  (`parent.UserConstructionScript`))