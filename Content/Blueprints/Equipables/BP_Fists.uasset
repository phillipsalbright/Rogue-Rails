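; BP_Fists is the player's unarmed melee equipable, punching whatever is within short range of the first-person camera.
; Action runs a Visibility line trace, applies point damage and plays a random left or right fist montage, gated by a cooldown that Tick counts down.
; Hits on BP_EnemyGuard spawn blood and call RestoreLastSlot on the player's inventory component, while other blocking hits spawn dust.
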(event `self.ReceiveTick`
  (params (DeltaSeconds :type "Float (single-precision)"))
  (`parent.ReceiveTick` DeltaSeconds)
  (if (> (`self.KnifeCooldown`) 0.0)
    (set `self.KnifeCooldown` (- (`self.KnifeCooldown`) DeltaSeconds))))

(fn `Action`
  (locals (FistsL :type "AnimMontage Object Reference" :default "/Script/Engine.AnimMontage'/Game/Models/Fists/AM_PunchL.AM_PunchL'") (FistsR :type "AnimMontage Object Reference" :default "/Script/Engine.AnimMontage'/Game/Models/Fists/AM_PunchR.AM_PunchR'"))
  (bind _firstpersoncamera (`/Game/Blueprints/Characters/BP_RRCharacter.FirstPersonCamera` (`self.Player Char`)))
  (bind _bp_inventorycomponent (`/Game/Blueprints/Characters/BP_RRCharacter.BP_InventoryComponent` (`self.Player Char`)))
  (bind _returnvalue (`SceneComponent.K2_GetComponentLocation` _firstpersoncamera))
  (`parent.Action`)
  (if (<= (`self.KnifeCooldown`) 0.0)
    (bind _outhit (`KismetSystemLibrary.LineTraceSingle` _returnvalue (+ _returnvalue (* (`SceneComponent.GetForwardVector` _firstpersoncamera) 200.0)) "TraceTypeQuery1"))
    (bind (_bblockinghit _binitialoverlap _time _distance _location _impactpoint _normal _impactnormal _physmat _hitactor) (`GameplayStatics.BreakHitResult` _outhit))
    (`GameplayStatics.ApplyPointDamage` _hitactor 1.0 (* _impactnormal -1.0) _outhit null null "/Engine/EngineDamageTypes/DmgTypeBP_Environmental.DmgTypeBP_Environmental_C")
    (cast `/Game/Blueprints/Characters/BP_EnemyGuard` _hitactor
      (:`then`
        (bind (_yaw _pitch) (`KismetMathLibrary.GetYawPitchFromVector` _impactnormal))
        (`NiagaraFunctionLibrary.SpawnSystemAtLocation` "/Game/VFX/NS_BloodSpray.NS_BloodSpray" _location (`KismetMathLibrary.MakeRotator` 0.0 _pitch _yaw) (0.3 0.3 0.3))
        (if (<= (`/Game/Blueprints/Inventory/BP_InventoryComponent.GetLastValidSLot` _bp_inventorycomponent) -1)
          (`/Game/Blueprints/Inventory/BP_InventoryComponent.RestoreLastSlot` _bp_inventorycomponent))
        (`/Game/Blueprints/Inventory/BP_InventoryComponent.RestoreLastSlot` _bp_inventorycomponent))
      (:`CastFailed`
        (if _bblockinghit
          (`NiagaraFunctionLibrary.SpawnSystemAtLocation` "/Game/VFX/NS_DustSpray.NS_DustSpray" _location (`KismetMathLibrary.MakeRotator` 0.0 _pitch _yaw) (0.5 0.5 0.5)))))
    (`AnimInstance.Montage_Play` (`SkeletalMeshComponent.GetAnimInstance` (`/Game/Blueprints/Characters/BP_RRCharacter.FistsMesh` (`self.Player Char`))) (select `bool` (`KismetMathLibrary.RandomBool`) :`false` (`local.FistsL`) :`true` (`local.FistsR`)) 1.5 "MontageLength" 0.0 true)
    (set `self.KnifeCooldown` 0.35)))

(fn `UserConstructionScript`
  (`parent.UserConstructionScript`))