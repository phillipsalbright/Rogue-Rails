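; BP_Lighter is an equippable lighter item that the player can open, close and use.
; AltAction calls AltFire, which plays an opening or closing montage on its skeletal mesh, then after a short delay flips the Closed state and shows or hides the Niagara effect, hidden at start.
; Action plays a use-object montage on the player's first-person mesh, but only while the lighter is open.
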(event `self.ReceiveBeginPlay`
  (`parent.ReceiveBeginPlay`)
  (`SceneComponent.SetHiddenInGame` (`self.Niagara`) true true))

(event `AltFire`
  (bind _niagara (`self.Niagara`))
  (bind _returnvalue (`SkeletalMeshComponent.GetAnimInstance` (`self.SkeletalMesh`)))
  (if (`self.Closed`)
    (`AnimInstance.Montage_Play` _returnvalue "/Game/Models/Items/AM_LighterOpening.AM_LighterOpening" 1.0 "MontageLength" 0.0 true)
    (`KismetSystemLibrary.Delay` 0.2)
    (set `self.Closed` false)
    (`SceneComponent.SetHiddenInGame` _niagara false true)
    (else
      (`AnimInstance.Montage_Play` _returnvalue "/Game/Models/Items/AM_LighterClose.AM_LighterClose" 1.0 "MontageLength" 0.0 true)
      (`KismetSystemLibrary.Delay` 0.2)
      (set `self.Closed` true)
      (`SceneComponent.SetHiddenInGame` _niagara true true))))

(fn `Action`
  (`parent.Action`)
  (if (not (`self.Closed`))
    (`AnimInstance.Montage_Play` (`SkeletalMeshComponent.GetAnimInstance` (`/Game/Blueprints/Characters/BP_RRCharacter.FirstPersonMesh` (`self.Player Char`))) "/Game/Models/Arms/AM_UseObject.AM_UseObject" 1.2 "MontageLength" 0.0 true)))

(fn `AltAction`
  (`parent.AltAction`)
  (`self.AltFire`))

(fn `UserConstructionScript`
  (`parent.UserConstructionScript`))