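; BP_Glock is an equipable silenced-sounding pistol that overrides its parent's Action to fire a hitscan shot.
; Action line-traces forward from the player's first-person camera, applies very high point damage to the hit actor, then plays the fire montage and shot sound.
; CheckForBullet always returns true, so ammo is unlimited and the out-of-ammo sound branch never runs.
; Equip and Unequip only call the parent.
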(fn `Action`
  (bind _firstpersoncamera (`/Game/Blueprints/Characters/BP_RRCharacter.FirstPersonCamera` (`self.Player Char`)))
  (bind _returnvalue (`SceneComponent.K2_GetComponentLocation` _firstpersoncamera))
  (`parent.Action`)
  (if (`self.CheckForBullet`)
    (bind _outhit (`KismetSystemLibrary.LineTraceSingle` _returnvalue (+ _returnvalue (* (`SceneComponent.GetForwardVector` _firstpersoncamera) 2000.0)) "TraceTypeQuery1"))
    (bind (_bblockinghit _binitialoverlap _time _distance _location _impactpoint _normal _impactnormal _physmat _hitactor) (`GameplayStatics.BreakHitResult` _outhit))
    (`GameplayStatics.ApplyPointDamage` _hitactor 1000000.0 (* _impactnormal -1.0) _outhit null null "/Engine/EngineDamageTypes/DmgTypeBP_Environmental.DmgTypeBP_Environmental_C")
    (`AnimInstance.Montage_Play` (`SkeletalMeshComponent.GetAnimInstance` (`self.GlockMesh`)) "/Game/Models/Weapons/Glock/AM_GLockFire.AM_GLockFire" 1.0 "MontageLength" 0.0 true)
    (`GameplayStatics.PlaySoundAtLocation` "/Game/Audio/Silenced_Pistol_Sound_Effect.Silenced_Pistol_Sound_Effect" (`SceneComponent.K2_GetComponentLocation` (`self.barrelpoint`)) (struct) 1.0 1.0 0.0 null null null null)
    (else
      (`GameplayStatics.PlaySoundAtLocation` "/Game/Audio/165660__pacmangamer__out-of-ammo-no-ammo.165660__pacmangamer__out-of-ammo-no-ammo" (`SceneComponent.K2_GetComponentLocation` (`self.barrelpoint`)) (struct) 1.0 1.0 0.0 null null null null))))

(fn `CheckForBullet`
  (returns (HasBullet :type Boolean))
  (return true))

(fn `Equip`
  (params (PlayerChar :type "/Game/Blueprints/Characters/BP_RRCharacter Object Reference"))
  (`parent.Equip` PlayerChar))

(fn `Unequip`
  (`parent.Unequip`))

(fn `UserConstructionScript`)