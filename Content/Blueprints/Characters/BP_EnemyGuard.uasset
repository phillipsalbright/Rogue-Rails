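; BP_EnemyGuard is an enemy guard character that investigates, shoots at the player and can be killed.
; Damage plays a reaction, reports the player's location to BP_GuardController, and is tripled while unalerted.
; Shoot is rate-limited and line-traces to the player, calling RemoveSlots on a hit; timers also end inspections.
; Death unpossesses and ragdolls the guard, then attaches a BP_Body pickup with an inventory item object.
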(event `self.ReceiveBeginPlay`
  (add `self.OnTakeAnyDamage` (delegate `OnTakeAnyDamage_Event`)))

(event `OnTakeAnyDamage_Event` :!signature `self.OnTakeAnyDamage`
  (params (DamagedActor :type "Actor Object Reference") (Damage :type "Float (single-precision)") (DamageType :type "DamageType Object Reference") (InstigatedBy :type "Controller Object Reference") (DamageCauser :type "Actor Object Reference"))
  (`|PlayMontage` (`self.Mesh`) "/Game/Models/SecurityGuard/AM_React.AM_React"
    (:`then`
      (bind _asbp_guard_controller (cast `/Game/Blueprints/Controlers/BP_GuardController` (`AIBlueprintHelperLibrary.GetAIController` self)))
      (`/Game/Blueprints/Controlers/BP_GuardController.MadeSound` _asbp_guard_controller (`self.K2_GetActorLocation` (`GameplayStatics.GetPlayerPawn` 0)))
      (if (`self.Alert`)
        (set `self.Health` (- (`self.Health`) Damage))
        (else
          (set `self.Health` (- (`self.Health`) (* Damage 3.0)))))
      (if (<= (`self.Health`) 0.0)
        (`self.Death`)))))

(event `self.ReceiveTick`
  (params (DeltaSeconds :type "Float (single-precision)"))
  (bind _inspectiontime (`self.InspectionTime`))
  (`|ExecutionSequence`
    (:`then_0`
      (if (> _inspectiontime 0.0)
        (bind _output_get (set `self.InspectionTime` (- _inspectiontime DeltaSeconds)))
        (if (<= _output_get 0.0)
          (set `self.Inspecting` false))))
    (:`then_1`
      (set `self.ShootingTImer` (- (`self.ShootingTImer`) DeltaSeconds)))))

(fn `Death`
  (locals (NewLocalVar :type "Controller Object Reference") (FreshKill :type Boolean :default false))
  (bind _mesh (`self.Mesh`))
  (bind _output_get (set `local.NewLocalVar` (`AIBlueprintHelperLibrary.GetAIController` self)))
  (bind _output_get_2 (set `local.FreshKill` (`KismetSystemLibrary.IsValid` _output_get)))
  (if _output_get_2
    (`Controller.UnPossess` _output_get))
  (`SkinnedMeshComponent.SetPhysicsAsset` (`self.Mesh`) "/Game/Models/SecurityGuard/PA_SecurityGuard.PA_SecurityGuard" true)
  (`PrimitiveComponent.SetSimulatePhysics` _mesh true)
  (`PrimitiveComponent.SetCollisionEnabled` _mesh "QueryAndPhysics")
  (`PrimitiveComponent.SetCollisionEnabled` (`self.CapsuleComponent`) "NoCollision")
  (`PrimitiveComponent.SetCollisionEnabled` (`self.BodyBox`) "NoCollision")
  (`PrimitiveComponent.SetCollisionEnabled` (`self.HeadBox`) "NoCollision")
  (if (`local.FreshKill`)
    (bind _returnvalue (`|GenericCreateObject` "/Game/Blueprints/Items/BP_ItemObject.BP_ItemObject_C" (make `IntPoint` 4 2) "/Game/Materials/M_Icon_Skull.M_Icon_Skull" "/Game/Materials/M_Icon_Skull_R.M_Icon_Skull_R" "/Game/Blueprints/Items/BP_Body.BP_Body_C" false null))
    (bind _returnvalue_2 (`|SpawnActorFromClass` "/Game/Blueprints/Items/BP_Body.BP_Body_C" (`KismetMathLibrary.MakeTransform` (0.0 0.0 0.0)) "Undefined" "MultiplyWithRoot" null _returnvalue null))
    (`self.K2_AttachToComponent` _returnvalue_2 (`self.PickupAnchor`) "None" "KeepRelative" "KeepRelative" "KeepRelative" true)
    (set `/Game/Blueprints/Items/BP_Body.AttachedEnemy` self _returnvalue_2)))

(fn `SetAlert`
  (params (NewParam :type Boolean))
  (bind _output_get (set `self.Alert` NewParam))
  (if _output_get
    (`NiagaraFunctionLibrary.SpawnSystemAttached` "/Game/VFX/NS_SpottedEffect.NS_SpottedEffect" (`self.Mesh`) "Head" (0.0 -150.0 0.0) (struct) "KeepRelativeOffset" true)))

(fn `Shoot`
  (if (< (`self.ShootingTImer`) 0.0)
    (`AnimInstance.Montage_Play` (`SkeletalMeshComponent.GetAnimInstance` (`self.Mesh`)) "/Game/Models/SecurityGuard/AM_GuardShoot.AM_GuardShoot" 1.0 "MontageLength" 0.0 false)
    (`AnimInstance.Montage_Play` (`SkeletalMeshComponent.GetAnimInstance` (`self.SkeletalMesh`)) "/Game/Models/Weapons/Glock/AM_GLockFire.AM_GLockFire" 1.0 "MontageLength" 0.0 true)
    (set `self.ShootingTImer` 1.0)
    (`GameplayStatics.PlaySoundAtLocation` "/Game/Audio/SilencedGUn.SilencedGUn" (`self.K2_GetActorLocation`) (struct) 1.0 1.0 0.0 null null null null)
    (bind _outhit (`KismetSystemLibrary.LineTraceSingle` :`Start` (`self.K2_GetActorLocation`) :`End` (`self.K2_GetActorLocation` (`GameplayStatics.GetPlayerCharacter` 0)) :`TraceChannel` "TraceTypeQuery2" :`DrawDebugType` "ForDuration"))
    (bind _asbp_rrcharacter (cast `/Game/Blueprints/Characters/BP_RRCharacter` (`.HitActor` (`GameplayStatics.BreakHitResult` _outhit))))
    (`/Game/Blueprints/Characters/BP_RRCharacter.RemoveSlots` _asbp_rrcharacter 1)))

(fn `StartInvestigation`
  (set `self.Inspecting` true)
  (set `self.InspectionTime` 10.0))

(fn `UserConstructionScript`)