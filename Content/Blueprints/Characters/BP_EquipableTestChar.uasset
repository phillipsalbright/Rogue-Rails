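; BP_EquipableTestChar is a test character Blueprint for switching between equipable weapons.
; Number keys 1, 2 and 3 call EquipWeapon with the bottle, Glock and knife Blueprints respectively.
; EquipWeapon is not defined in these graphs, and BeginPlay and the construction script only call their parent versions.
; Leftover unconnected nodes for equipping the bottle and a delayed knife swap never run.
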(event `self.ReceiveBeginPlay`
  (`parent.ReceiveBeginPlay`))

(event `Key|One`
  (params (Key :type "Key Structure"))
  (:`Pressed`
    (`self.EquipWeapon` "/Game/Blueprints/Equipables/BP_Bottle.BP_Bottle_C")))

(event `Key|Two`
  (params (Key :type "Key Structure"))
  (:`Pressed`
    (`self.EquipWeapon` "/Game/Blueprints/Equipables/BP_Glock.BP_Glock_C")))

(event `Key|Three`
  (params (Key :type "Key Structure"))
  (:`Pressed`
    (`self.EquipWeapon` "/Game/Blueprints/Equipables/BP_Knife.BP_Knife_C")))

(fn `UserConstructionScript`
  (`parent.UserConstructionScript`))