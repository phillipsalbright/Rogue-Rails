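; Game mode for the RR main level that opens the game on a popup and stocks the player's starting inventory.
; BeginPlay waits a tick, shows WBP_Popup, pauses the game, switches input to UI-only with a visible cursor, then calls AddItems.
; AddItems builds BP_ItemObjects for an equippable Glock, bullets and an equippable knife, with grid sizes and rotated icons, and adds them to the character's inventory component.
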(event `self.ReceiveBeginPlay`
  (bind _returnvalue (`GameplayStatics.GetPlayerController` 0))
  (`parent.ReceiveBeginPlay`)
  (`KismetSystemLibrary.DelayUntilNextTick`)
  (bind _returnvalue_2 (`|CreateWidget` "/Game/UI/WBP_Popup.WBP_Popup_C"))
  (`UserWidget.AddToPlayerScreen` _returnvalue_2 0)
  (`GameplayStatics.SetGamePaused` true)
  (`WidgetBlueprintLibrary.SetInputMode_UIOnlyEx` _returnvalue null)
  (set `PlayerController.bShowMouseCursor` true _returnvalue)
  (`self.AddItems`))

(fn `AddItems`
  (locals (Inventory :type "/Game/Blueprints/Inventory/BP_InventoryComponent Object Reference"))
  (bind _asbp_rrcharacter (cast `/Game/Blueprints/Characters/BP_RRCharacter` (`GameplayStatics.GetPlayerCharacter` 0)))
  (set `local.Inventory` (`/Game/Blueprints/Characters/BP_RRCharacter.BP_InventoryComponent` _asbp_rrcharacter))
  (bind _returnvalue (`|GenericCreateObject` "/Game/Blueprints/Items/BP_ItemObject.BP_ItemObject_C" (make `IntPoint` 3 2) "/Game/Materials/M_Icon_Glock.M_Icon_Glock" "/Game/Materials/M_Icon_Glock_R.M_Icon_Glock_R" "/Game/Blueprints/Items/BP_GlockPickup.BP_GlockPickup_C" true "/Game/Blueprints/Equipables/BP_Glock.BP_Glock_C" "Glock"))
  (`/Game/Blueprints/Inventory/BP_InventoryComponent.TryAddItem` (`local.Inventory`) _returnvalue)
  (bind _returnvalue_2 (`|GenericCreateObject` "/Game/Blueprints/Items/BP_ItemObject.BP_ItemObject_C" (make `IntPoint` 1 1) "/Game/Materials/M_Icon_Bullet.M_Icon_Bullet" "/Game/Materials/M_Icon_Bullet_Rotated.M_Icon_Bullet_Rotated" "/Game/Blueprints/Items/BP_BulletPickup.BP_BulletPickup_C" false null "Bullet"))
  (`/Game/Blueprints/Inventory/BP_InventoryComponent.TryAddItem` (`local.Inventory`) _returnvalue_2)
  (bind _returnvalue_3 (`|GenericCreateObject` "/Game/Blueprints/Items/BP_ItemObject.BP_ItemObject_C" (make `IntPoint` 1 1) "/Game/Materials/M_Icon_Bullet.M_Icon_Bullet" "/Game/Materials/M_Icon_Bullet_Rotated.M_Icon_Bullet_Rotated" "/Game/Blueprints/Items/BP_BulletPickup.BP_BulletPickup_C" false null "Bullet"))
  (`/Game/Blueprints/Inventory/BP_InventoryComponent.TryAddItem` (`local.Inventory`) _returnvalue_3)
  (bind _returnvalue_4 (`|GenericCreateObject` "/Game/Blueprints/Items/BP_ItemObject.BP_ItemObject_C" (make `IntPoint` 1 1) "/Game/Materials/M_Icon_Bullet.M_Icon_Bullet" "/Game/Materials/M_Icon_Bullet_Rotated.M_Icon_Bullet_Rotated" "/Game/Blueprints/Items/BP_BulletPickup.BP_BulletPickup_C" false null "Bullet"))
  (`/Game/Blueprints/Inventory/BP_InventoryComponent.TryAddItem` (`local.Inventory`) _returnvalue_4)
  (bind _returnvalue_5 (`|GenericCreateObject` "/Game/Blueprints/Items/BP_ItemObject.BP_ItemObject_C" (make `IntPoint` 3 1) "/Game/Materials/M_Icon_Knife.M_Icon_Knife" "/Game/Materials/M_Icon_Knife_rotated.M_Icon_Knife_rotated" "/Game/Blueprints/Items/BP_KnifePickup.BP_KnifePickup_C" true "/Game/Blueprints/Equipables/BP_Knife.BP_Knife_C" "Knife"))
  (`/Game/Blueprints/Inventory/BP_InventoryComponent.TryAddItem` (`local.Inventory`) _returnvalue_5))

(fn `UserConstructionScript`
  (`parent.UserConstructionScript`))