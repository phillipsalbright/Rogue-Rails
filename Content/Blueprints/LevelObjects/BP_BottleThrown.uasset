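; BP_BottleThrown is a thrown bottle that shatters on impact and alerts nearby guards to the noise.
; When its static mesh hits something, it plays a glass shatter sound at its location.
; It then finds BP_EnemyGuard actors overlapping its sphere, calls MadeSound on each one's BP_GuardController with the impact location, and destroys itself.
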(event `self.StaticMesh.OnComponentHit`
  (params (HitComponent :type "PrimitiveComponent Object Reference") (OtherActor :type "Actor Object Reference") (OtherComp :type "PrimitiveComponent Object Reference") (NormalImpulse :type "Vector Structure") (Hit :type "HitResult Structure (by ref)"))
  (`GameplayStatics.PlaySoundAtLocation` "/Game/Audio/GlassShatter.GlassShatter" (`self.K2_GetActorLocation` self) (struct) 1.0 1.0 0.55 null null null null)
  (for _array_element (`PrimitiveComponent.GetOverlappingActors` (`self.Sphere`) "/Game/Blueprints/Characters/BP_EnemyGuard.BP_EnemyGuard_C")
    (bind _asbp_guard_controller (cast `/Game/Blueprints/Controlers/BP_GuardController` (`AIBlueprintHelperLibrary.GetAIController` _array_element))
      (:`then`
        (`/Game/Blueprints/Controlers/BP_GuardController.MadeSound` _asbp_guard_controller (`self.K2_GetActorLocation` self)))
      (:`CastFailed`
        (`KismetSystemLibrary.PrintString` "Hello"))))
  (`self.K2_DestroyActor`))

(fn `UserConstructionScript`)