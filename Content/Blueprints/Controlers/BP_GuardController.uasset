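; AI controller for BP_EnemyGuard that patrols, chases and shoots the player, and investigates noises.
; AI perception sets the target, sight flag, last known position and memory timer, and drives the guard's alert state.
; Tick runs the logic without a behavior tree: shoot in range, chase or search, then resume patrol when the timer expires.
; MadeSound sends an unsighted guard to investigate; unpossessing stops Tick and expires the controller.
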(event `self.ReceivePossess`
  (params (PossessedPawn :type "Pawn Object Reference"))
  (bind _asbp_enemy_guard (cast `/Game/Blueprints/Characters/BP_EnemyGuard` PossessedPawn))
  (set `self.GuardChar` _asbp_enemy_guard))

(event `self.ReceiveBeginPlay`
  (bind _guardchar (`self.GuardChar`))
  (set `self.PatrolPoints` (`/Game/Blueprints/Characters/BP_EnemyGuard.PatrolPoints` _guardchar))
  (`KismetArrayLibrary.Array_Add` (`self.PatrolPoints`) (`self.K2_GetActorLocation` _guardchar))
  (set `self.PatrolPointIndex` 0))

(event `self.ReceiveTick`
  (params (DeltaSeconds :type "Float (single-precision)"))
  (bind _canseeplayer (`self.CanSeePlayer`))
  (bind _patrolpoints (`self.PatrolPoints`))
  (bind _patrolpointindex (`self.PatrolPointIndex`))
  (bind _target (`self.Target`))
  (bind _output (`|GetArrayItem` _patrolpoints _patrolpointindex))
  (`|ExecutionSequence`
    (:`then_0`
      (if (or _canseeplayer (> (`self.float PlayerTimer`) 0.0))
        (if (and (< (`KismetMathLibrary.VSize` (- (`self.K2_GetActorLocation` _target) (`self.K2_GetActorLocation` (`self.GuardChar`)))) 1000.0) _canseeplayer)
          (`self.StopMovement`)
          (`self.K2_SetFocus` _target)
          (`/Game/Blueprints/Characters/BP_EnemyGuard.Shoot` (`self.GuardChar`))
          (elif (`self.CanSeePlayer`)
            (`self.K2_ClearFocus`)
            (`|AIMoveTo` null (0.0 0.0 0.0) _target 900.0)
            (else
              (`self.K2_ClearFocus`)
              (`|AIMoveTo` null (`self.LastPlayerPoint`) null))))))
    (:`then_1`
      (if (not (`self.CanSeePlayer`))
        (bind _output_get (set `self.float PlayerTimer` (- (`self.float PlayerTimer`) DeltaSeconds)))
        (if (< _output_get 0.0)
          (set `self.Target` null)
          (if (not (`/Game/Blueprints/Characters/BP_EnemyGuard.Inspecting` (`self.GuardChar`)))
            (`self.Alerted` false)
            (if (< (`KismetMathLibrary.VSize` (- (`self.K2_GetActorLocation` (`self.GuardChar`)) _output)) 50.0)
              (bind _output_get_2 (set `self.PatrolPointIndex` (mod (+ _patrolpointindex 1) (- (`KismetArrayLibrary.Array_Length` _patrolpoints) 1))))
              (`KismetSystemLibrary.PrintString` (`KismetStringLibrary.Conv_IntToString` _output_get_2))
              (else
                (`|AIMoveTo` null _output null)))))))))

(event `self.ReceiveUnPossess`
  (params (UnpossessedPawn :type "Pawn Object Reference"))
  (`self.SetActorTickEnabled` false)
  (`self.SetLifeSpan` 1.0))

(event `self.AIPerception.OnTargetPerceptionInfoUpdated`
  (params (UpdateInfo :type "ActorPerceptionUpdateInfo Structure (by ref)"))
  (if (`.bSuccessfullySensed` (break `AIStimulus` (`.Stimulus` (break `ActorPerceptionUpdateInfo` UpdateInfo))))
    (bind _asbp_rrcharacter (cast `/Game/Blueprints/Characters/BP_RRCharacter` UpdateInfo_Target))
    (set `self.Target` _asbp_rrcharacter)
    (set `self.CanSeePlayer` true)
    (set `self.float PlayerTimer` 10.0)
    (`self.Alerted` true)
    (else
      (bind _asbp_rrcharacter_2 (cast `/Game/Blueprints/Characters/BP_RRCharacter` UpdateInfo_Target))
      (set `self.LastPlayerPoint` (`self.K2_GetActorLocation` _asbp_rrcharacter_2))
      (if (== _asbp_rrcharacter_2 (`self.Target`))
        (set `self.CanSeePlayer` false)
        (set `self.float PlayerTimer` 10.0)))))

(fn `Alerted`
  (params (NewParam :type Boolean))
  (`/Game/Blueprints/Characters/BP_EnemyGuard.SetAlert` (`self.GuardChar`) NewParam))

(fn `MadeSound`
  (params (Location :type "Vector Structure"))
  (if (not (`self.CanSeePlayer`))
    (set `self.float PlayerTimer` -1.0)
    (`self.MoveToLocation` Location 20.0 true true false true null)
    (`/Game/Blueprints/Characters/BP_EnemyGuard.StartInvestigation` (`self.GuardChar`))
    (`KismetSystemLibrary.PrintString` "Heard something...")
    (`self.Alerted` false)
    (`self.Alerted` true)))

(fn `UserConstructionScript`)